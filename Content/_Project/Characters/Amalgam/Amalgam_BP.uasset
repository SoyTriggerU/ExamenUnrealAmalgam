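; Amalgam playable character Blueprint that sets up health, armor and shield and registers three skill components: bomb, glide and jet jump.
; Input actions fire the skills and ultimate; holding Jump glides and disables the bomb until release.
; While jet jump thrusts, movement input is ignored and Tick pushes the actor along control rotation with sweep.
; An unfinished position-recall rewind remains, with its playback logic disconnected.
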(event `self.ReceiveBeginPlay`
  (bind _amalgam_da_bomb_skill_bpc (`self.Amalgam_Da_Bomb_Skill_BPC`))
  (bind _amalgam_glide_skill_bpc (`self.Amalgam_Glide_Skill_BPC`))
  (bind _jet_jump_amalgama_skill_bpc (`self.Jet_Jump_Amalgama_Skill_BPC`))
  (`parent.ReceiveBeginPlay`)
  (`|ExecutionSequence`
    (:`then_0`
      (`self.InitializeHealth` (make `/Game/_Project/CommonSystems/HealthSystem/HealthData` 125.0 125.0 50.0 50.0 50.0 50.0)))
    (:`then_1`
      (`/Game/_Project/CommonSystems/Character_Skills/Character_Skill_BP.Initialize` _amalgam_da_bomb_skill_bpc self "E")
      (`KismetArrayLibrary.Array_Add` (`self.Skills`) _amalgam_da_bomb_skill_bpc))
    (:`then_2`
      (`/Game/_Project/CommonSystems/Character_Skills/Character_Skill_BP.Initialize` _amalgam_glide_skill_bpc self "SPACE")
      (`KismetArrayLibrary.Array_Add` (`self.Skills`) _amalgam_glide_skill_bpc))
    (:`then_3`
      (`/Game/_Project/CommonSystems/Character_Skills/Character_Skill_BP.Initialize` _jet_jump_amalgama_skill_bpc self "LSHIFT")
      (`KismetArrayLibrary.Array_Add` (`self.Skills`) _jet_jump_amalgama_skill_bpc))))

(event `EnhancedInput|/Game/_Project/CommonSystems/Input/Skill_0`
  (params (ActionValue :type Boolean) (ElapsedSeconds :type "Float (double-precision)") (TriggeredSeconds :type "Float (double-precision)") (InputAction :type "InputAction Object Reference" :default "/Game/_Project/CommonSystems/Input/Skill_0.Skill_0"))
  (:`Started`
    (`/Game/_Project/CommonSystems/Character_Skills/Character_Skill_BP.Fire` (`self.Jet_Jump_Amalgama_Skill_BPC`))))

(event `EnhancedInput|/Game/_Project/CommonSystems/Input/Skill_1`
  (params (ActionValue :type Boolean) (ElapsedSeconds :type "Float (double-precision)") (TriggeredSeconds :type "Float (double-precision)") (InputAction :type "InputAction Object Reference" :default "/Game/_Project/CommonSystems/Input/Skill_1.Skill_1"))
  (bind _amalgam_da_bomb_skill_bpc (`self.Amalgam_Da_Bomb_Skill_BPC`))
  (:`Started`
    (set `/Game/_Project/Characters/Amalgam/Skills/Da_Bomb/Amalgam_Da_Bomb_Skill_BPC.SpawnPoint` (`SceneComponent.K2_GetComponentToWorld` (`self.GrenadeSpawnPoint`)) _amalgam_da_bomb_skill_bpc)
    (`/Game/_Project/CommonSystems/Character_Skills/Character_Skill_BP.Fire` _amalgam_da_bomb_skill_bpc)))

(event `EnhancedInput|/Game/_Project/CommonSystems/Input/Ultimate`
  (params (ActionValue :type Boolean) (ElapsedSeconds :type "Float (double-precision)") (TriggeredSeconds :type "Float (double-precision)") (InputAction :type "InputAction Object Reference" :default "/Game/_Project/CommonSystems/Input/Ultimate.Ultimate"))
  (:`Started`
    (`/Game/_Project/CommonSystems/Character_Ultimate/Ultimate_BP.Fire` (`self.Ultimate`))))

(event `EnhancedInput|/Game/_Project/CommonSystems/Input/Jump`
  (params (ActionValue :type Boolean) (ElapsedSeconds :type "Float (double-precision)") (TriggeredSeconds :type "Float (double-precision)") (InputAction :type "InputAction Object Reference" :default "/Game/_Project/CommonSystems/Input/Jump.Jump"))
  (bind _amalgam_da_bomb_skill_bpc (`self.Amalgam_Da_Bomb_Skill_BPC`))
  (bind _amalgam_glide_skill_bpc (`self.Amalgam_Glide_Skill_BPC`))
  (bind _amalgam_glide_skill_bpc_2 (`self.Amalgam_Glide_Skill_BPC`))
  (bind _amalgam_glide_skill_bpc_3 (`self.Amalgam_Glide_Skill_BPC`))
  (:`Triggered`
    (set `/Game/_Project/Characters/Amalgam/Skills/Glide/Amalgam_Glide_Skill_BPC.IsHoldingSpace` true _amalgam_glide_skill_bpc_2)
    (`/Game/_Project/CommonSystems/Character_Skills/Character_Skill_BP.Fire` _amalgam_glide_skill_bpc_2)
    (`/Game/_Project/CommonSystems/Character_Skills/Character_Skill_BP.SetEnabled` _amalgam_da_bomb_skill_bpc false))
  (:`Canceled`
    (set `/Game/_Project/Characters/Amalgam/Skills/Glide/Amalgam_Glide_Skill_BPC.IsHoldingSpace` false _amalgam_glide_skill_bpc_3)
    (`/Game/_Project/CommonSystems/Character_Skills/Character_Skill_BP.Finish` _amalgam_glide_skill_bpc_3)
    (`/Game/_Project/CommonSystems/Character_Skills/Character_Skill_BP.SetEnabled` _amalgam_da_bomb_skill_bpc true))
  (:`Completed`
    (set `/Game/_Project/Characters/Amalgam/Skills/Glide/Amalgam_Glide_Skill_BPC.IsHoldingSpace` false _amalgam_glide_skill_bpc)
    (`/Game/_Project/CommonSystems/Character_Skills/Character_Skill_BP.Finish` _amalgam_glide_skill_bpc)
    (`/Game/_Project/CommonSystems/Character_Skills/Character_Skill_BP.SetEnabled` _amalgam_da_bomb_skill_bpc true)))

(event `EnhancedInput|/Game/_Project/CommonSystems/Input/Move`
  (params (ActionValue :type "Vector2D Structure") (ElapsedSeconds :type "Float (double-precision)") (TriggeredSeconds :type "Float (double-precision)") (InputAction :type "InputAction Object Reference" :default "/Game/_Project/CommonSystems/Input/Move.Move"))
  (bind (_x _y) (`KismetMathLibrary.BreakVector2D` ActionValue))
  (:`Triggered`
    (if (not (`/Game/_Project/Characters/Amalgam/Skills/Jet_Jump/Jet_Jump_Amalgama_Skill_BPC.IsThrusting` (`self.Jet_Jump_Amalgama_Skill_BPC`)))
      (`self.AddMovementInput` (`SceneComponent.GetForwardVector` (`self.CapsuleComponent`)) _x)
      (`self.AddMovementInput` (`SceneComponent.GetRightVector` (`self.CapsuleComponent`)) _y))))

(event `self.ReceiveTick`
  (params (DeltaSeconds :type "Float (single-precision)"))
  (`parent.ReceiveTick` DeltaSeconds)
  (if (`/Game/_Project/Characters/Amalgam/Skills/Jet_Jump/Jet_Jump_Amalgama_Skill_BPC.IsThrusting` (`self.Jet_Jump_Amalgama_Skill_BPC`))
    (`self.K2_AddActorWorldOffset` (* (`KismetMathLibrary.GetForwardVector` (`self.GetControlRotation`)) (* (`KismetMathLibrary.Conv_DoubleToVector` DeltaSeconds) 600.0)) true)))

(event `CustomEvent`
  (`KismetSystemLibrary.K2_SetTimerDelegate` (delegate `StoreTRansform`) (`self.RecallSaveTime`)))

(event `StoreTRansform`
  (if (not (`self.IsRecalling`))
    (`KismetArrayLibrary.Array_Insert` (`self.RecallPosition`) (`self.GetTransform`))
    (`KismetArrayLibrary.Array_Resize` (`self.RecallPosition`) (`KismetMathLibrary.Round` (/ (`self.RecallMaxSaveTime`) (`self.RecallSaveTime`))))))

(event `Key|LeftShift`
  (params (Key :type "Key Structure")))

(fn `UserConstructionScript`
  (`parent.UserConstructionScript`))